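; Health component for the loop scene that resets health on begin play and offers heal, damage, reset and clamped set functions.
; Health and death state live in BP_LoopGameInstance, whose OnHealthChanged event fires after each change.
; TakeDamage also plays a sound through the game mode's music manager and calls OnDeath when dead.
; Its Min against zero, rather than Max, leaves health at zero or below after any hit.
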(event `self.ReceiveBeginPlay`
  (bind _gameinstanceref (`self.GameInstanceRef`))
  (bind _gameinstanceref_2 (`self.GameInstanceRef`))
  (`|ExecutionSequence`
    (:`then_0`
      (bind _asbp_loop_game_instance (cast `/Game/Game/Blueprint/Pawn/BP_LoopGameInstance` (`GameplayStatics.GetGameInstance`)))
      (set `self.GameInstanceRef` _asbp_loop_game_instance)
      (bind _asbp_custom_game_mode (cast `/Game/Game/Blueprint/BP_CustomGameMode` (`GameplayStatics.GetGameMode`)))
      (set `self.GameModeRef` _asbp_custom_game_mode))
    (:`then_1`
      (set `/Game/Game/Blueprint/Pawn/BP_LoopGameInstance.CurrentHealth` (`/Game/Game/Blueprint/Pawn/BP_LoopGameInstance.MaxHealth` _gameinstanceref) _gameinstanceref))
    (:`then_2`
      (`/Game/Game/Blueprint/Pawn/BP_LoopGameInstance.OnHealthChanged` _gameinstanceref_2 (`/Game/Game/Blueprint/Pawn/BP_LoopGameInstance.CurrentHealth` _gameinstanceref_2) (`/Game/Game/Blueprint/Pawn/BP_LoopGameInstance.MaxHealth` _gameinstanceref_2)))))

(fn `Heal`
  (params (amount :type Integer))
  (bind _gameinstanceref (`self.GameInstanceRef`))
  (bind _gameinstanceref_2 (`self.GameInstanceRef`))
  (`|ExecutionSequence`
    (:`then_0`
      (if (`/Game/Game/Blueprint/Pawn/BP_LoopGameInstance.IsDead` (`self.GameInstanceRef`))
        (return)))
    (:`then_1`
      (set `/Game/Game/Blueprint/Pawn/BP_LoopGameInstance.CurrentHealth` (`KismetMathLibrary.Min` (+ (`/Game/Game/Blueprint/Pawn/BP_LoopGameInstance.CurrentHealth` _gameinstanceref_2) (`local.amount`)) (`/Game/Game/Blueprint/Pawn/BP_LoopGameInstance.MaxHealth` _gameinstanceref_2)) _gameinstanceref_2))
    (:`then_2`
      (`/Game/Game/Blueprint/Pawn/BP_LoopGameInstance.OnHealthChanged` _gameinstanceref (`/Game/Game/Blueprint/Pawn/BP_LoopGameInstance.CurrentHealth` _gameinstanceref) (`/Game/Game/Blueprint/Pawn/BP_LoopGameInstance.MaxHealth` _gameinstanceref)))))

(fn `ResetHealth`
  (bind _gameinstanceref (`self.GameInstanceRef`))
  (bind _gameinstanceref_2 (`self.GameInstanceRef`))
  (`|ExecutionSequence`
    (:`then_0`
      (set `/Game/Game/Blueprint/Pawn/BP_LoopGameInstance.CurrentHealth` (`/Game/Game/Blueprint/Pawn/BP_LoopGameInstance.MaxHealth` _gameinstanceref_2) _gameinstanceref_2))
    (:`then_1`
      (`/Game/Game/Blueprint/Pawn/BP_LoopGameInstance.OnHealthChanged` _gameinstanceref (`/Game/Game/Blueprint/Pawn/BP_LoopGameInstance.CurrentHealth` _gameinstanceref) (`/Game/Game/Blueprint/Pawn/BP_LoopGameInstance.MaxHealth` _gameinstanceref)))))

(fn `SetCurrentHealth`
  (params (Health :type Integer))
  (bind _gameinstanceref (`self.GameInstanceRef`))
  (bind _gameinstanceref_2 (`self.GameInstanceRef`))
  (`|ExecutionSequence`
    (:`then_0`
      (set `/Game/Game/Blueprint/Pawn/BP_LoopGameInstance.CurrentHealth` (`KismetMathLibrary.Clamp` Health 0 (`/Game/Game/Blueprint/Pawn/BP_LoopGameInstance.MaxHealth` _gameinstanceref_2)) _gameinstanceref_2))
    (:`then_1`
      (`/Game/Game/Blueprint/Pawn/BP_LoopGameInstance.OnHealthChanged` _gameinstanceref (`/Game/Game/Blueprint/Pawn/BP_LoopGameInstance.CurrentHealth` _gameinstanceref) (`/Game/Game/Blueprint/Pawn/BP_LoopGameInstance.MaxHealth` _gameinstanceref)))))

(fn `TakeDamage`
  (params (Amount :type Integer))
  (bind _gameinstanceref (`self.GameInstanceRef`))
  (bind _gameinstanceref_2 (`self.GameInstanceRef`))
  (bind _gameinstanceref_3 (`self.GameInstanceRef`))
  (bind _bpc_musicmanager (`/Game/Game/Blueprint/BP_CustomGameMode.BPC_MusicManager` (`self.GameModeRef`)))
  (`|ExecutionSequence`
    (:`then_0`
      (if (`/Game/Game/Blueprint/Pawn/BP_LoopGameInstance.IsDead` (`self.GameInstanceRef`))
        (return)))
    (:`then_1`
      (set `/Game/Game/Blueprint/Pawn/BP_LoopGameInstance.CurrentHealth` (`KismetMathLibrary.Min` (- (`/Game/Game/Blueprint/Pawn/BP_LoopGameInstance.CurrentHealth` _gameinstanceref_3) (`local.amount`))) _gameinstanceref_3))
    (:`then_2`
      (`/Game/Game/Blueprint/Pawn/BP_LoopGameInstance.OnHealthChanged` _gameinstanceref (`/Game/Game/Blueprint/Pawn/BP_LoopGameInstance.CurrentHealth` _gameinstanceref) (`/Game/Game/Blueprint/Pawn/BP_LoopGameInstance.MaxHealth` _gameinstanceref)))
    (:`then_3`
      (if (!= _bpc_musicmanager null)
        (`/Game/Game/Blueprint/Managers/LoopScene/BPC_MusicManager.PlayTakeDamageSound` _bpc_musicmanager)))
    (:`then_4`
      (if (`/Game/Game/Blueprint/Pawn/BP_LoopGameInstance.IsDead` _gameinstanceref_2)
        (`/Game/Game/Blueprint/Pawn/BP_LoopGameInstance.OnDeath` _gameinstanceref_2)))))