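; BP_DialogueCell is a cell Blueprint that runs a dialogue sequence for the pawn that activates it.
; Activate resets its dialogue component to the starting row, pushes that row's character and long text to the pawn's DialogueRef, then starts the dialogue.
; Each Update call either exits the dialogue when the component reports it finished, or reads the next row and displays it through PlayDialogue.
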(event `/Game/Game/Blueprint/Cells/BPI_Activable.Activate`
  (params (Pawn :type "/Game/Game/Blueprint/Pawn/BP_Pawn Object Reference"))
  (`/Game/Game/Blueprint/Dialogue/BPC_DialogueManager.ResetRow` (`self.BPC_DialogueComponent`))
  (`self.PlayDialogue` Pawn)
  (`/Game/Game/Widget/BPW_DialogueUI.StartDialogue` (`/Game/Game/Blueprint/Pawn/BP_Pawn.DialogueRef` Pawn)))

(event `/Game/Game/Blueprint/Cells/BPI_Activable.Update`
  (params (Pawn :type "/Game/Game/Blueprint/Pawn/BP_Pawn Object Reference"))
  (bind _bpc_dialoguecomponent (`self.BPC_DialogueComponent`))
  (bind _isfinished (`/Game/Game/Blueprint/Dialogue/BPC_DialogueManager.IsDialogueFinished` _bpc_dialoguecomponent))
  (if _isfinished
    (`/Game/Game/Widget/BPW_DialogueUI.ExitDialogue` (`/Game/Game/Blueprint/Pawn/BP_Pawn.DialogueRef` Pawn))
    (else
      (`/Game/Game/Blueprint/Dialogue/BPC_DialogueManager.ReadNextRow` _bpc_dialoguecomponent)
      (`self.PlayDialogue` Pawn))))

(fn `PlayDialogue`
  (params (Pawn :type "/Game/Game/Blueprint/Pawn/BP_Pawn Object Reference"))
  (bind _bpc_dialoguecomponent (`self.BPC_DialogueComponent`))
  (`/Game/Game/Blueprint/Dialogue/BPC_DialogueManager.GetCurrentDialogueRowData` _bpc_dialoguecomponent)
  (bind _charactername (`/Game/Game/Blueprint/Dialogue/BPC_DialogueManager.GetCharacterFromCurrentRow` _bpc_dialoguecomponent))
  (bind _dialoguelong (`/Game/Game/Blueprint/Dialogue/BPC_DialogueManager.GetDialogueLongFromCurrentRow` _bpc_dialoguecomponent))
  (`/Game/Game/Widget/BPW_DialogueUI.UpdateDialogue` (`/Game/Game/Blueprint/Pawn/BP_Pawn.DialogueRef` Pawn) _charactername _dialoguelong))

(fn `UserConstructionScript`
  (`parent.UserConstructionScript`))