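; BP_TreasureCell is a cell Blueprint for a treasure tied to a quest, with a visual that it refreshes on BeginPlay and every Tick.
; UpdateTreasureVisibility checks that the visual and quest are set, computes visibility from quest-active and collected flags, then forces both the visual and ShouldBeVisible to true regardless.
; ActivateQuest only stores the current pawn; its remaining branch is empty.
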(event `self.ReceiveBeginPlay`
  (`parent.ReceiveBeginPlay`)
  (`self.UpdateTreasureVisibility`))

(event `self.ReceiveTick`
  (params (DeltaSeconds :type "Float (single-precision)"))
  (`parent.ReceiveTick` DeltaSeconds)
  (`self.UpdateTreasureVisibility`))

(fn `ActivateQuest`
  (params (CurrentPawn :type "/Game/Game/Blueprint/Pawn/BP_Pawn Object Reference"))
  (`|ExecutionSequence`
    (:`then_0`
      (set `self.BpPawnRef` CurrentPawn))
    (:`then_1`
      (if true
        (`|ExecutionSequence`)))))

(fn `UpdateTreasureVisibility`
  (locals (shouldBeVisible :type Boolean))
  (if (and (!= (`self.TreasureVisual`) null) (!= (`self.questToComplete`) null))
    (`|ExecutionSequence`
      (:`then_0`
        (set `local.shouldBeVisible` (and (`/Game/Game/Blueprint/Managers/LoopScene/BPC_QuestManager.QuestIsActive` (`self.questToComplete`)) (`self.hasBeenCollected`))))
      (:`then_1`
        (`SceneComponent.SetVisibility` (`self.TreasureVisual`) true false)
        (set `local.shouldBeVisible` true)))))

(fn `UserConstructionScript`
  (`parent.UserConstructionScript`))