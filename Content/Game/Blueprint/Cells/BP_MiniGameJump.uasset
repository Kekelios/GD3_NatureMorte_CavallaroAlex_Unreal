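; BP_MiniGameJump is a cell actor that sends the player into the parkour jump minigame.
; When activated by a BP_Pawn, it sets that pawn's health to 100 through its health system component, then opens Map_Parkour.
; Both steps require the game instance to be BP_LoopGameInstance, which is also cached on BeginPlay.
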(event `self.ReceiveBeginPlay`
  (`parent.ReceiveBeginPlay`)
  (bind _asbp_loop_game_instance (cast `/Game/Game/Blueprint/Pawn/BP_LoopGameInstance` (`GameplayStatics.GetGameInstance`)))
  (set `self.As BP Loop Game Instance` _asbp_loop_game_instance))

(event `self.Activate`
  (params (Pawn :type "/Game/Game/Blueprint/Pawn/BP_Pawn Object Reference"))
  (bind _asbp_pawn (cast `/Game/Game/Blueprint/Pawn/BP_Pawn` Pawn))
  (cast `/Game/Game/Blueprint/Pawn/BP_LoopGameInstance` (`GameplayStatics.GetGameInstance`))
  (`/Game/Game/Blueprint/Managers/LoopScene/BPC_HealthSystem.SetCurrentHealth` (`/Game/Game/Blueprint/Pawn/BP_Pawn.BPC_HealthSystem` _asbp_pawn) 100)
  (`GameplayStatics.OpenLevelBySoftObjectPtr` "/Game/Game/Map/Map_Parkour.Map_Parkour"))

(fn `UserConstructionScript`
  (`parent.UserConstructionScript`))