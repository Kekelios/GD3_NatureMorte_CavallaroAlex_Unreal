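; BP_TrapCell is a trap cell whose ActivateTrap function is meant to damage the pawn passed to it.
; It exits early if already triggered and repeat damage is off, though this graph never sets HasBeenTriggered.
; It then sets the pawn's BPCHealthSystem to None, caches that reference, and calls TakeDamage with DamageAmount if it passes the check.
; BeginPlay and construction only call the parent.
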(event `self.ReceiveBeginPlay`
  (`parent.ReceiveBeginPlay`))

(fn `ActivateTrap`
  (params (CurrentPawn :type "/Game/Game/Blueprint/Pawn/BP_Pawn Object Reference"))
  (locals (HealthSystemRef :type "/Game/Game/Blueprint/Managers/LoopScene/BPC_HealthSystem Object Reference"))
  (`|ExecutionSequence`
    (:`then_0`
      (if (and (not (`self.canDamageMultipleTimes`)) (`self.hasBeenTriggered`))
        (return)))
    (:`then_1`
      (bind _output_get (set `/Game/Game/Blueprint/Pawn/BP_Pawn.BPC_HealthSystem` null (`local.CurrentPawn`)))
      (set `local.HealthSystemRef` _output_get))
    (:`then_2`
      (if (!= (`local.HealthSystemRef`) null)
        (`/Game/Game/Blueprint/Managers/LoopScene/BPC_HealthSystem.TakeDamage` (`local.HealthSystemRef`) (`self.damageAmount`))))))

(fn `UserConstructionScript`
  (`parent.UserConstructionScript`))