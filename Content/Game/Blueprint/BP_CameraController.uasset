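; Orbit camera controller that follows the pawn target, defaulting to the first BP_Pawn found at BeginPlay.
; Each Tick updates the follow point with an offset and optional smoothing, then applies right-click mouse rotation and scroll zoom, both clamped.
; It then places the actor at zoom distance from that point and turns it to look at it.
; Player input can be enabled or disabled while following continues, and the view can be reset.
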(event `self.ReceiveBeginPlay`
  (bind _asbp_custom_game_mode (cast `/Game/Game/Blueprint/BP_CustomGameMode` (`GameplayStatics.GetGameMode`)))
  (bind _output_get (set `self.GameModeRef` _asbp_custom_game_mode))
  (`|ExecutionSequence`
    (:`then_0`
      (if (== (`self.PawnTarget`) null)
        (bind _returnvalue (`GameplayStatics.GetActorOfClass` "/Game/Game/Blueprint/Pawn/BP_Pawn.BP_Pawn_C"))
        (if (!= _returnvalue null)
          (set `self.PawnTarget` _returnvalue))))
    (:`then_2`
      (set `self.CurrentZoom` (`self.DefaultZoom `))
      (if (!= (`self.PawnTarget`) null)
        (set `self.CurrentTargetPosition` (`self.K2_GetActorLocation` (`self.PawnTarget`)))))))

(event `self.ReceiveTick`
  (params (DeltaSeconds :type "Float (single-precision)"))
  (`self.LateUpdate`))

(fn `DisableControls`
  (set `self.CanControl` false))

(fn `EnableControls`
  (set `self.CanControl` true))

(fn `HandleRotation`
  (locals (mouseDelta :type "Vector2D Structure"))
  (bind (_mousedelta_x _mousedelta_y) (`KismetMathLibrary.BreakVector2D` (`local.mouseDelta`)))
  (bind _mousedelta_x_2 (`KismetMathLibrary.BreakVector2D` (`local.mouseDelta`)))
  (if (`|GetInputActionValue`)
    (set `local.mouseDelta` (`KismetMathLibrary.MakeVector2D` (`self.GetInputAxisKeyValue`) (`self.GetInputAxisKeyValue`)))
    (set `self.CurrentRotationY` (- (`self.CurrentRotationY`) (* (* _mousedelta_x_2 (`self.rotationSpeed`)) (`GameplayStatics.GetWorldDeltaSeconds`))))
    (set `self.CurrentRotationX` (- (`self.CurrentRotationX`) (* (* _mousedelta_y (`self.rotationSpeed`)) (`GameplayStatics.GetWorldDeltaSeconds`))))
    (set `self.CurrentRotationX` (`KismetMathLibrary.FClamp` (`self.CurrentRotationX`) (`self.MinVerticalAngle`) (`self.MaxVerticalAngle `)))))

(fn `HandleZoom`
  (locals (scrollValue :type "Float (double-precision)"))
  (set `local.scrollValue` (`self.GetInputAxisKeyValue`))
  (if (!= (`local.scrollValue`) 0.0)
    (set `self.CurrentZoom` (- (`self.CurrentZoom`) (* (`local.scrollValue`) (`self.ZoomSpeed `))))
    (set `self.CurrentZoom` (`KismetMathLibrary.FClamp` (`self.CurrentZoom`) (`self.MinZoom `) (`self.MaxZoom `)))))

(fn `LateUpdate`
  (`|ExecutionSequence`
    (:`then_0`
      (if (== (`self.PawnTarget`) null)
        (return)))
    (:`then_1`
      (`self.UpdateTargetPosition`))
    (:`then_2`
      (if (`self.CanControl`)
        (`|ExecutionSequence`
          (:`then_0`
            (`self.HandleRotation`))
          (:`then_1`
            (`self.HandleZoom`)))))
    (:`then_3`
      (`self.UpdateCameraPosition`))))

(fn `ResetCamera`
  (set `self.CurrentRotationY` 0.0)
  (set `self.CurrentRotationX` 38.25)
  (set `self.CurrentZoom` (`self.DefaultZoom `)))

(fn `UpdateCameraPosition`
  (locals (Rotation :type "Rotator Structure") (Direction :type "Vector Structure") (DesiredPosition :type "Vector Structure"))
  (set `local.Rotation` (`KismetMathLibrary.MakeRotator` 0.0 (* (`self.CurrentRotationX`) -1.0) (* (`self.CurrentRotationY`) -1.0)))
  (set `local.Direction` (`KismetMathLibrary.NegateVector` (`KismetMathLibrary.GetForwardVector` (`local.Rotation`))))
  (set `local.DesiredPosition` (+ (* (`local.Direction`) (`self.CurrentZoom`)) (`self.CurrentTargetPosition`)))
  (`self.K2_SetActorLocation` (`local.DesiredPosition`))
  (`self.K2_SetActorRotation` (`KismetMathLibrary.FindLookAtRotation` (`self.K2_GetActorLocation`) (`self.CurrentTargetPosition`))))

(fn `UpdateTargetPosition`
  (locals (DesiredPosition :type "Vector Structure"))
  (set `local.DesiredPosition` (+ (`self.K2_GetActorLocation` (`self.PawnTarget`)) (`self.TargetOffset`)))
  (if (`self.SmoothFollow`)
    (set `self.CurrentTargetPosition` (`KismetMathLibrary.VLerp` (`self.CurrentTargetPosition`) (`local.DesiredPosition`) (* (`self.FollowSpeed`) (`GameplayStatics.GetWorldDeltaSeconds`))))
    (else
      (set `self.CurrentTargetPosition` (`local.DesiredPosition`)))))

(fn `UserConstructionScript`)