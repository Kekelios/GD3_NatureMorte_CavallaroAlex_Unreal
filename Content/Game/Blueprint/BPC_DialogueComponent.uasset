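; BPC_DialogueComponent is a dialogue component that reads lines from a DataTable and exposes their contents.
; The current row number, converted to a Name, serves as the key to fetch and return a row.
; Getters expose the long dialogue and character from the stored CurrentDialogueRow, and a negative NextRow marks the dialogue as finished.
; ReadNextRow is an empty stub, and nothing here assigns CurrentDialogueRow.
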(fn `GetCharacterFromCurrentRow`
  (returns (CharacterName :type String))
  ; On récupère le character
  (return (`.Character_5_C826C5B14C5EB937AA60FDB2562CB49F` (break `/Game/Game/Blueprint/ST_DialogueRowData` (`self.CurrentDialogueRow`)))))

(fn `GetCurrentDialogueRowData`
  (returns (RowData :type "/Game/Game/Blueprint/ST_DialogueRowData Structure"))
  ;[0.002643 1 0.1862 0.5] Récupère la ligne de dialogue actuelle (CurrentDialogeRow)
  (bind _returnvalue (`|GetDataTableRow` (`self.DialogueDatatable`) (`KismetStringLibrary.Conv_StringToName` (`KismetStringLibrary.Conv_IntToString` (`self.CurrentRowNumber`))))
    (:`then`
      (return _returnvalue))))

(fn `GetDialogueLongFromCurrentRow`
  (returns (DialogueLong :type String))
  ; On récupère le dialogue
  (return (`.DialogeLong_7_104610BD4A2CF5DFFBE5B5A9C8918877` (break `/Game/Game/Blueprint/ST_DialogueRowData` (`self.CurrentDialogueRow`)))))

(fn `IsDialogueFinished`
  (returns (IsFinished :type Boolean))
  (return (< (`.NextRow_11_6EED0AF34209D386BFCAE397C7C54B6A` (break `/Game/Game/Blueprint/ST_DialogueRowData` (`self.CurrentDialogueRow`))) 0)))

(fn `ReadNextRow`)