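; BP_Coins is a collectible coin for the Pac-Man minigame, picked up when BP_ThirdPersonCharacter overlaps its trigger component.
; On pickup it increments the character's FoodScore, plays a quiet coin sound and prints the new score.
; It then calls CoinsCollected on the BP_ThirdPersonGameMode, found through GetAllActorsOfClass, and destroys itself.
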(event `self.ReceiveBeginPlay`)

(event `self.CoinPickUptRIGGER.OnComponentBeginOverlap`
  (params (OverlappedComponent :type "PrimitiveComponent Object Reference") (OtherActor :type "Actor Object Reference") (OtherComp :type "PrimitiveComponent Object Reference") (OtherBodyIndex :type Integer) (bFromSweep :type Boolean) (SweepResult :type "HitResult Structure (by ref)"))
  (bind _asbp_third_person_character (cast `/Game/Game/Blueprint/PacManMiniGame/BP_ThirdPersonCharacter` OtherActor))
  (bind _output_get (set `self.ThirdPersonRef` _asbp_third_person_character))
  (bind _output_get_2 (set `/Game/Game/Blueprint/PacManMiniGame/BP_ThirdPersonCharacter.FoodScore` (+ (`/Game/Game/Blueprint/PacManMiniGame/BP_ThirdPersonCharacter.FoodScore` _output_get) 1) _output_get))
  (`GameplayStatics.SpawnSoundAtLocation` "/Game/Game/Blueprint/PacManMiniGame/Coins.Coins" (0.0 0.0 0.0) (struct) 0.1 1.0 0.0 null null)
  (`KismetSystemLibrary.PrintString` (`KismetStringLibrary.Conv_IntToString` _output_get_2))
  (bind _outactors (`GameplayStatics.GetAllActorsOfClass` "/Game/ThirdPerson/Blueprints/BP_ThirdPersonGameMode.BP_ThirdPersonGameMode_C"))
  (`/Game/ThirdPerson/Blueprints/BP_ThirdPersonGameMode.CoinsCollected` _outactors)
  (`self.K2_DestroyActor`))

(fn `UserConstructionScript`)