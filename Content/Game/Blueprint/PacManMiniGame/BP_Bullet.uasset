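; BP_Bullet is a flashing pickup in the Pac-Man minigame that triggers scared mode, acting like a power pellet.
; From BeginPlay, a FlipFlop and Delay loop endlessly toggles the coin mesh's visibility.
; When BP_ThirdPersonCharacter overlaps the trigger, it plays a coin sound at world origin, calls ActivateScaredMode on BP_ThirdPersonGameMode found via GetAllActorsOfClass, then destroys itself.
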(event `self.ReceiveBeginPlay`
  (`self.Flashing`))

(event `self.CoinPickUptRIGGER.OnComponentBeginOverlap`
  (params (OverlappedComponent :type "PrimitiveComponent Object Reference") (OtherActor :type "Actor Object Reference") (OtherComp :type "PrimitiveComponent Object Reference") (OtherBodyIndex :type Integer) (bFromSweep :type Boolean) (SweepResult :type "HitResult Structure (by ref)"))
  (bind _asbp_third_person_character (cast `/Game/Game/Blueprint/PacManMiniGame/BP_ThirdPersonCharacter` OtherActor))
  (set `self.ThirdPersonRef` _asbp_third_person_character)
  (`GameplayStatics.SpawnSoundAtLocation` "/Game/Game/Blueprint/PacManMiniGame/Coins.Coins" (0.0 0.0 0.0) (struct) 0.1 1.0 0.0 null null)
  (bind _outactors (`GameplayStatics.GetAllActorsOfClass` "/Game/ThirdPerson/Blueprints/BP_ThirdPersonGameMode.BP_ThirdPersonGameMode_C"))
  (`/Game/ThirdPerson/Blueprints/BP_ThirdPersonGameMode.Activate Scared Mode` _outactors)
  (`self.K2_DestroyActor`))

(event `Flashing`
  (`/Engine/EditorBlueprintResources/StandardMacros.FlipFlop` :!label _label
    (:`A`
      (`SceneComponent.SetVisibility` (`self.SM_Coins`) false false)
      (`KismetSystemLibrary.Delay` 2.0)
      (goto _label))
    (:`B`
      (`SceneComponent.SetVisibility` (`self.SM_Coins`) true false)
      (`KismetSystemLibrary.Delay` 2.0)
      (`SceneComponent.SetVisibility` (`self.SM_Coins`) false false)
      (goto _label))))

(fn `UserConstructionScript`)