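; BP_Mummy is an enemy in the PacMan minigame that wanders the level and threatens the player.
; After a random start delay it roams in a self-restarting AIMoveTo loop over random reachable points.
; When PawnSensing sees a pawn and ChasePlayer is set, it pursues the player, resuming roaming shortly after a failed move.
; Sphere overlap with the player plays a scream, then destroys the mummy if IsScared, otherwise deducts GameInstance health and calls Death.
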(event `self.ReceiveBeginPlay`
  (`KismetSystemLibrary.Delay` (`KismetMathLibrary.FClamp` (`KismetMathLibrary.RandomFloat`) 2.5 7.0))
  (`self.RandomRoam`))

(event `RandomRoam`
  (`|AIMoveTo` self (`NavigationSystemV1.K2_GetRandomReachablePointInRadius` (`self.K2_GetActorLocation`) 3000.0 null null) null
    (:`OnSuccess`
      _)
    (:`OnFail`
      _))
  (`self.RandomRoam`))

(event `self.PawnSensing.OnSeePawn`
  (params (Pawn :type "Pawn Object Reference"))
  (if (`self.ChasePlayer`)
    (bind _asbp_third_person_character (cast `/Game/Game/Blueprint/PacManMiniGame/BP_ThirdPersonCharacter` (`GameplayStatics.GetPlayerCharacter` 0)))
    (`|AIMoveTo` self (0.0 0.0 0.0) _asbp_third_person_character
      (:`OnFail`
        (`KismetSystemLibrary.RetriggerableDelay` 2.0)
        (`self.RandomRoam`)))))

(event `self.Sphere.OnComponentBeginOverlap`
  (params (OverlappedComponent :type "PrimitiveComponent Object Reference") (OtherActor :type "Actor Object Reference") (OtherComp :type "PrimitiveComponent Object Reference") (OtherBodyIndex :type Integer) (bFromSweep :type Boolean) (SweepResult :type "HitResult Structure (by ref)"))
  (bind _asbp_third_person_character (cast `/Game/Game/Blueprint/PacManMiniGame/BP_ThirdPersonCharacter` OtherActor))
  (`GameplayStatics.PlaySoundAtLocation` "/Game/Game/SD/universfield-male-death-scream-horror-352706.universfield-male-death-scream-horror-352706" (0.0 0.0 0.0) (struct) 0.5 1.0 0.0 null null null null)
  (bind _output_get (set `self.CharacterRef` _asbp_third_person_character))
  (if (`self.IsScared`)
    (`self.K2_DestroyActor`)
    (else
      (bind _gameinstanceref (`/Game/Game/Blueprint/PacManMiniGame/BP_ThirdPersonCharacter.GameInstanceRef` _output_get))
      (set `/Game/Game/Blueprint/Pawn/BP_LoopGameInstance.CurrentHealth` (- (`/Game/Game/Blueprint/Pawn/BP_LoopGameInstance.CurrentHealth` _gameinstanceref) 25) _gameinstanceref)
      (`/Game/Game/Blueprint/PacManMiniGame/BP_ThirdPersonCharacter.Death` _output_get))))

(fn `UserConstructionScript`)