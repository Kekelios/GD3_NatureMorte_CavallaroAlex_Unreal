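; BP_Pawn is the player's board-game piece, moving cell by cell along the board and triggering the cell it lands on.
; TryMoving re-calls itself every 0.2 seconds to animate each step of a roll, then ActivateCell messages the final cell.
; The current cell number lives in BP_LoopGameInstance, and BeginPlay uses it to place the pawn via BoardRef.
; BeginPlay also creates the dialogue widget, while UpdateCell forwards updates to the current cell.
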(event `self.ReceiveBeginPlay`
  (bind _asbp_loop_game_instance (cast `/Game/Game/Blueprint/Pawn/BP_LoopGameInstance` (`GameplayStatics.GetGameInstance`)))
  (set `self.GameInstanceRef` _asbp_loop_game_instance)
  (`self.MoveToCell`)
  (bind _returnvalue (`|CreateWidget` "/Game/Game/Widget/BPW_DialogueUI.BPW_DialogueUI_C"))
  (bind _output_get (set `self.DialogueRef` _returnvalue))
  (`UserWidget.AddToViewport` _output_get 0)
  (set `/Game/Game/Widget/BPW_DialogueUI.PawnRef` self _returnvalue))

(event `TryMoving`
  (params (Value :type Integer))
  ;[1 1 1 0.5] Animation for each movement until the roll number is over
  (`self.TryingMoving` 1)
  (if (> Value 1)
    (`KismetSystemLibrary.Delay` 0.2)
    (`self.TryMoving` (- Value 1))
    (else
      (`self.ActivateCell` self))))

(fn `ActivateCell`
  (bind _cell (`/Game/Game/Blueprint/Cells/BP_Board.GetCellByNumber` (`self.BoardRef`) (`/Game/Game/Blueprint/Pawn/BP_LoopGameInstance.CellNumber` (`self.GameInstanceRef`))))
  (message `/Game/Game/Blueprint/Cells/BPI_Activable.Activate` _cell self))

(fn `MoveToCell`
  (bind _cell (`/Game/Game/Blueprint/Cells/BP_Board.GetCellByNumber` (`self.BoardRef`) (`/Game/Game/Blueprint/Pawn/BP_LoopGameInstance.CellNumber` (`self.GameInstanceRef`))))
  (bind (_returnvalue_location _returnvalue_rotation) (`KismetMathLibrary.BreakTransform` (`self.GetTransform` _cell)))
  (`self.K2_SetActorLocationAndRotation` (+ _returnvalue_location (0.0 0.0 50.0)) _returnvalue_rotation))

(fn `TryingMoving`
  (params (Value :type Integer))
  (bind _gameinstanceref (`self.GameInstanceRef`))
  (bind _cell (`/Game/Game/Blueprint/Cells/BP_Board.GetNextCellToMove` (`self.BoardRef`) (+ Value (`/Game/Game/Blueprint/Pawn/BP_LoopGameInstance.CellNumber` _gameinstanceref))))
  (set `/Game/Game/Blueprint/Pawn/BP_LoopGameInstance.CellNumber` _cell _gameinstanceref)
  (`self.MoveToCell`))

(fn `UpdateCell`
  (bind _cell (`/Game/Game/Blueprint/Cells/BP_Board.GetCellByNumber` (`self.BoardRef`) (`/Game/Game/Blueprint/Pawn/BP_LoopGameInstance.CellNumber` (`self.GameInstanceRef`))))
  (message `/Game/Game/Blueprint/Cells/BPI_Activable.Update` _cell self))

(fn `UserConstructionScript`)