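; Dialogue manager component that tracks and reads the current conversation from a DataTable.
; Rows are looked up by number and chained through each entry's NextRow, with a negative value marking the end.
; A second flow starts a passed-in dialogue, fires a started event and advances a line index toward choices or ending.
; That flow is unfinished: ShowChoices, EndDialogue and DisplayCurrentLine are empty.
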(fn `DisplayCurrentLine`)

(fn `EndDialogue`)

(fn `GetCharacterFromCurrentRow`
  (returns (CharacterName :type String))
  ; On récupère le character
  (return (`.Character_5_C826C5B14C5EB937AA60FDB2562CB49F` (break `/Game/Game/Blueprint/Dialogue/ST_DialogueData` (`self.CurrentDialogue`)))))

(fn `GetCurrentDialogueRowData`
  (returns (RowData :type "/Game/Game/Blueprint/Dialogue/ST_DialogueData Structure"))
  ;[0.002643 1 0.1862 0.5] Récupère la ligne de dialogue actuelle (CurrentDialogeRow)
  (bind _returnvalue (`|GetDataTableRow` (`self.DialogueDatatable`) (`KismetStringLibrary.Conv_StringToName` (`KismetStringLibrary.Conv_IntToString` (`self.CurrentRowNumber`))))
    (:`then`
      (bind _output_get (set `self.CurrentDialogue` _returnvalue))
      (return _output_get))))

(fn `GetDialogueLongFromCurrentRow`
  (returns (DialogueLong :type String))
  ; On récupère le dialogue
  (return (`.DialogueText_12_104610BD4A2CF5DFFBE5B5A9C8918877` (break `/Game/Game/Blueprint/Dialogue/ST_DialogueData` (`self.CurrentDialogue`)))))

(fn `IsDialogueFinished`
  (returns (IsFinished :type Boolean))
  (return (< (`.NextRow_27_FA96E5A341D94C329F48F19C17503CC5` (break `/Game/Game/Blueprint/Dialogue/ST_DialogueData` (`self.CurrentDialogue`))) 0)))

(fn `ReadNextRow`
  (set `self.CurrentRowNumber` (`.NextRow_27_FA96E5A341D94C329F48F19C17503CC5` (break `/Game/Game/Blueprint/Dialogue/ST_DialogueData` (`self.CurrentDialogue`))))
  (`self.GetCurrentDialogueRowData`))

(fn `ResetRow`
  (set `self.CurrentRowNumber` 0))

(fn `ShowChoices`)

(fn `ShowNextLine`
  (bind (_rownumber _character _dialoguetext _haschoice _choicescount) (break `/Game/Game/Blueprint/Dialogue/ST_DialogueData` (`self.CurrentDialogue`)))
  (`|ExecutionSequence`
    (:`then_0`
      (if (or (`self.waitingForChoice`) (not (`self.isDialogueActive`)))
        (return)))
    (:`then_1`
      (set `self.currentLineIndex` (+ (`self.currentLineIndex`) 1)))
    (:`then_2`
      (if (>= (`self.currentLineIndex`) (`.RowNumber_2_793B1BFC4767D77A0BFD798A61797E13` (break `/Game/Game/Blueprint/Dialogue/ST_DialogueData` (`self.CurrentDialogue`))))
        (if (and _haschoice (> _choicescount 0))
          (`self.ShowChoices`)
          (else
            (`|ExecutionSequence`
              (:`then_0`
                (`self.EndDialogue`))
              (:`then_1`
                (`self.DisplayCurrentLine`)))))))))

(fn `StartDialogue`
  (params (dialogue :type "/Game/Game/Blueprint/Dialogue/ST_DialogueData Structure"))
  (`|ExecutionSequence`
    (:`then_0`
      (set `self.CurrentDialogue` dialogue))
    (:`then_1`
      (set `self.currentLineIndex` 0))
    (:`then_2`
      (set `self.isDialogueActive` true))
    (:`then_3`
      (set `self.waitingForChoice` false))
    (:`then_4`
      (`self.OnDialogueStarted`))))